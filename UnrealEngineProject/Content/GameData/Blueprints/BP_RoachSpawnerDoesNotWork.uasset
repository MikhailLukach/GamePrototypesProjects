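; Roach spawner actor that periodically spawns BP_MovingFoodItem actors at its own transform, passing along its FoodItemAsset.
; A looping timer started on BeginPlay calls Spawn, which adds items until AmountInLevel reaches a small cap.
; The count decrements only in the spawner's own Destroyed event and nothing binds to spawned items' destruction, so removed items never free up slots.
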(event Custom|Spawn
  (if (< (Variables|Default|GetamountInLevel) 5.0)
    (Game|SpawnActorfromClass "/Game/GameData/Blueprints/Interactable/BP_MovingFoodItem.BP_MovingFoodItem_C" (Transformation|GetActorTransform self) "Undefined" "MultiplyWithRoot" 0 true (Variables|Default|GetfoodItemAsset) 0)
    (Variables|Default|SetamountInLevel (+ (Variables|Default|GetamountInLevel) 1.0))))

(event EventBeginPlay
  (Utilities|Time|SetTimerbyFunctionName 0 "Spawn" 1e+01 true))

(event EventDestroyed
  (Variables|Default|SetamountInLevel (- (Variables|Default|GetamountInLevel) 1.0)))

(fn ConstructionScript)