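; Player character Blueprint for a prison game, handling movement, grabbing and dropping objects, interactions, and resource stats.
; A short sphere trace in front of the character, using separate channels for grab and interact, messages the hit actor; grabbed objects attach to the hands.
; Interaction state toggles an extra Enhanced Input mapping context.
; Custom events adjust cigar currency, sentence and prison unrest, with affordability checks for meat and vegetables.
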(event Custom|Grab
  (params (ObjectToGrab :type BP%20Grabable%20Object%20Reference))
  ;[1 1 1] Grabs object and sets its position to the player's hand
  (bind _output_get (Variables|Default|SetgrabbedObject ObjectToGrab))
  (Transformation|AttachComponentToComponent _output_get (Variables|Default|Gethands) "None" "KeepWorld" "KeepWorld" "KeepWorld" true)
  (Components|MoveComponentTo (Variables|/Script/Engine.Actor|GetRootComponent (Variables|Default|GetgrabbedObject)) "0, 0, 0" "0, 0, 0" false false 0.2 false))

(event Custom|SetIsInteracting
  (params (IsInteracting :type Boolean) (InteractingObject :type BPI%20Interactable%20Interface))
  (bind _returnvalue (Game|GetPlayerController 0))
  (bind _returnvalue_2 (PlayerController|LocalPlayerSubsystems|GetEnhancedInputLocalPlayerSubsystem _returnvalue))
  ;[1 1 1] Sets that player is currently interacting with object
  (Variables|Default|SetisInteracting IsInteracting)
  (Variables|Default|SetinteractingObject InteractingObject)
  (if (Variables|Default|GetisInteracting)
    (Input|AddMappingContext _returnvalue_2 "/Game/GameData/Inputs/IMC_Interaction.IMC_Interaction" 0 "(bIgnoreAllPressedKeysUntilRelease=True,bForceImmediately=False,bNotifyUserSettings=False)")
    (else
      (Input|RemoveMappingContext _returnvalue_2 "/Game/GameData/Inputs/IMC_Interaction.IMC_Interaction" "(bIgnoreAllPressedKeysUntilRelease=True,bForceImmediately=False,bNotifyUserSettings=False)"))))

(event Custom|IncrementHalfCigars
  ;[1 1 1] Callable incrementing and decrementing custom events to manage the game's systems
  (Variables|GameAmounts|SetcigarsAmount (+ (Variables|GameAmounts|GetcigarsAmount) 50)))

(event Custom|IncrementHalfPrisonUnrest
  ;[1 1 1] Callable incrementing and decrementing custom events to manage the game's systems
  (Variables|GameAmounts|SetprisonUnrest (+ (Variables|GameAmounts|GetprisonUnrest) 0.1)))

(event Custom|StopInteraction
  ;[1 1 1] Tells object that player has stopped interacting with them
  (Default|StopInteraction (Variables|Default|GetinteractingObject)))

(event Custom|IncrementCigars
  ;[1 1 1] Callable incrementing and decrementing custom events to manage the game's systems
  (Variables|GameAmounts|SetcigarsAmount (+ (Variables|GameAmounts|GetcigarsAmount) 100)))

(event Custom|IncrementPrisonUnrest
  ;[1 1 1] Callable incrementing and decrementing custom events to manage the game's systems
  (Variables|GameAmounts|SetprisonUnrest (+ (Variables|GameAmounts|GetprisonUnrest) 0.2)))

(event Custom|DecrementPrisonUnrest
  ;[1 1 1] Callable incrementing and decrementing custom events to manage the game's systems
  (Variables|GameAmounts|SetprisonUnrest (- (Variables|GameAmounts|GetprisonUnrest) 0.2)))

(event Custom|DecrementVegPrice
  ;[1 1 1] Callable incrementing and decrementing custom events to manage the game's systems
  (Variables|GameAmounts|SetcigarsAmount (- (Variables|GameAmounts|GetcigarsAmount) 25)))

(event Custom|DecrementMeatPrice
  ;[1 1 1] Callable incrementing and decrementing custom events to manage the game's systems
  (Variables|GameAmounts|SetcigarsAmount (- (Variables|GameAmounts|GetcigarsAmount) 50)))

(event Custom|DecrementSentence
  ;[1 1 1] Callable incrementing and decrementing custom events to manage the game's systems
  (Variables|GameAmounts|SetsentenceAmount (- (Variables|GameAmounts|GetsentenceAmount) 5)))

(event Custom|IncrementSentence
  ;[1 1 1] Callable incrementing and decrementing custom events to manage the game's systems
  (Variables|GameAmounts|SetsentenceAmount (+ (Variables|GameAmounts|GetsentenceAmount) 5)))

(event Input|EnhancedActionEvents|EnhancedInputActionIA_GrabDrop
  (params (ActionValue :type Boolean) (ElapsedSeconds :type Float%20%28double-precision%29) (TriggeredSeconds :type Float%20%28double-precision%29) (InputAction :type Input%20Action%20Object%20Reference :default "/Game/GameData/Inputs/IA_GrabDrop.IA_GrabDrop"))
  (bind (_returnvalue _grabbedobject) (CallFunction|GetGrabbedObject))
  ;[1 1 1] Check if hit, either allow player to grab object or drop the object held
  (:Started
    (bind (_returnvalue_2 _outhit) (CallFunction|FindObjecttoInteractwith "TraceTypeQuery3"))
    (if _returnvalue_2
      (Class|BPIInteractable|GrabDrop(Message) (.HitActor (Collision|BreakHitResult _outhit)) self)
      (elif _returnvalue
        (Default|Drop _grabbedobject)
        (Variables|Default|SetgrabbedObject 0)))))

(event Input|EnhancedActionEvents|EnhancedInputActionIA_Movement
  (params (ActionValue :type Vector%202D%20Structure) (ElapsedSeconds :type Float%20%28double-precision%29) (TriggeredSeconds :type Float%20%28double-precision%29) (InputAction :type Input%20Action%20Object%20Reference :default "/Game/GameData/Inputs/IA_Movement.IA_Movement"))
  ;[1 1 1] Adds movement input to Pawn
  (Pawn|Input|AddMovementInput (Math|Conversions|ToVector(Vector2D) ActionValue) 1.0 false))

(event Input|EnhancedActionEvents|EnhancedInputActionIA_StartInteraction
  (params (ActionValue :type Boolean) (ElapsedSeconds :type Float%20%28double-precision%29) (TriggeredSeconds :type Float%20%28double-precision%29) (InputAction :type Input%20Action%20Object%20Reference :default "/Game/GameData/Inputs/IA_StartInteraction.IA_StartInteraction"))
  ;[1 1 1] Performs interaction action for the player
  (:Started
    (if (Variables|Default|GetisInteracting)
      (CallFunction|StopInteraction)
      (else
        (bind (_returnvalue _outhit) (CallFunction|FindObjecttoInteractwith "TraceTypeQuery4"))
        (if _returnvalue
          (Class|BPIInteractable|Interact(Message) (.HitActor (Collision|BreakHitResult _outhit)) self))))))

(event Input|EnhancedActionEvents|EnhancedInputActionIA_StopInteraction
  (params (ActionValue :type Boolean) (ElapsedSeconds :type Float%20%28double-precision%29) (TriggeredSeconds :type Float%20%28double-precision%29) (InputAction :type Input%20Action%20Object%20Reference :default "/Game/GameData/Inputs/IA_StopInteraction.IA_StopInteraction"))
  ;[1 1 1] Sets that player has stopped interacting with the object
  (:Started
    (CallFunction|StopInteraction)))

(event EventBeginPlay)

(event Collision|EventActorBeginOverlap
  (params (OtherActor :type Actor%20Object%20Reference)))

(event EventTick
  (params (DeltaSeconds :type Float%20%28single-precision%29)))

(fn ConstructionScript)

(fn GetGrabbedObject
  (bind _grabbedobject (Variables|Default|GetgrabbedObject))
  (return (Utilities|IsValid _grabbedobject) _grabbedobject))

(fn FindObjecttoInteractwith
  (params (TraceChannel :type ETraceTypeQuery%20Enum :default "TraceTypeQuery1"))
  (bind _returnvalue (Transformation|GetActorForwardVector))
  (bind _returnvalue_2 (Transformation|GetActorLocation))
  (bind _returnvalue_3 (* _returnvalue 5e+01))
  (bind _returnvalue_4 (+ _returnvalue_3 _returnvalue_2))
  (bind (_x _y _z) (Math|Vector|BreakVector _returnvalue_4))
  (bind (_outhit _returnvalue_5) (Collision|SphereTraceByChannel (Math|Vector|MakeVector _x _y (+ _z -5e+01)) (Math|Vector|MakeVector _x _y (+ _z 1e+01)) 3e+01 TraceChannel false (Utilities|Array|MakeArray (Variables|Default|GetgrabbedObject)) "ForDuration"))
  (return _returnvalue_5 _outhit))

(fn CheckifEnoughforMeat
  (if (>= (Variables|GameAmounts|GetcigarsAmount) 50)
    (return true)
    (else
      (return false))))

(fn CheckifEnoughforVeg
  (if (>= (Variables|GameAmounts|GetcigarsAmount) 25)
    (return true)
    (else
      (return false))))