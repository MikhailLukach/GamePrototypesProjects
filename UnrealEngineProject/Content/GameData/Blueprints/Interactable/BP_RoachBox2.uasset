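; BP_RoachBox2 is an interactable box that dispenses a roach ingredient into the player's hands, with no cigs required.
; GrabDrop plays the box-opening sound, then defers to the parent logic if a placed object can be grabbed or, with nothing placed, the player is already holding something.
; For an empty-handed player at an empty box, it spawns a BP_MovingFoodItem from its FoodItemAsset and immediately hands it over.
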(event EventGrabDrop
  (params (Player :type BP%20Character%20Object%20Reference))
  ;[1 1 1] Spawns roach ingredient in to player's hands when they interact with the box, no amount of cigs is necessary
  (bind _outactors (Actor|GetAllActorsOfClass "/Game/MySoundEffectPlayer.MySoundEffectPlayer_C"))
  (Class|SoundEffectPlayer|PlaySoundEffect (Utilities|Array|Get(acopy) _outactors) "/Game/GameData/WAVs/SW_OpenBox.SW_OpenBox" (Transformation|GetActorLocation))
  (bind _placedobject (Variables|Default|GetplacedObject)
    (:then
      (if (Default|CanbeGrabbed _placedobject Player)
        (|CallParentFunction Player :!label _label)))
    (:else
      (if (.ReturnValue (Default|GetGrabbedObject Player))
        (goto _label)
        (else
          (bind _returnvalue (Game|SpawnActorfromClass "/Game/GameData/Blueprints/Interactable/BP_MovingFoodItem.BP_MovingFoodItem_C" (Transformation|GetActorTransform) "Undefined" "MultiplyWithRoot" 0 true (Variables|FoodBox|GetfoodItemAsset) 0))
          (Default|GrabDrop _returnvalue Player))))))

(fn ConstructionScript
  (|CallParentFunction))