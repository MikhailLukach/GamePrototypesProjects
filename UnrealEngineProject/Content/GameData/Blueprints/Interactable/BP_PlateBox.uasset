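; BP_PlateBox is an interactable plate dispenser that hands the player a new plate.
; Its GrabDrop event plays a box-opening sound through the first MySoundEffectPlayer found in the level.
; With nothing placed on it and an empty-handed player, it spawns a BP_Plate and calls that plate's GrabDrop.
; Otherwise it defers to the parent's grab/drop logic, unless the placed object cannot be grabbed.
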(event EventGrabDrop
  (params (Player :type BP%20Character%20Object%20Reference))
  ;[1 1 1] Gives a plate to the player when they interact with the plate box
  (bind _outactors (Actor|GetAllActorsOfClass "/Game/MySoundEffectPlayer.MySoundEffectPlayer_C"))
  (Class|SoundEffectPlayer|PlaySoundEffect (Utilities|Array|Get(acopy) _outactors) "/Game/GameData/WAVs/SW_OpenBox.SW_OpenBox" (Transformation|GetActorLocation))
  (bind _placedobject (Variables|Default|GetplacedObject)
    (:then
      (if (Default|CanbeGrabbed _placedobject Player)
        (|CallParentFunction Player :!label _label)))
    (:else
      (if (.ReturnValue (Default|GetGrabbedObject Player))
        (goto _label)
        (else
          (bind _returnvalue (Game|SpawnActorfromClass "/Game/GameData/Blueprints/Interactable/KitchenWare/BP_Plate.BP_Plate_C" (Transformation|GetActorTransform) "Undefined" "MultiplyWithRoot" 0 0))
          (Default|GrabDrop _returnvalue Player))))))

(fn ConstructionScript
  (|CallParentFunction))