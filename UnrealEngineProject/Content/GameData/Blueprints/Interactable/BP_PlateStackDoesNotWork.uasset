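; Interactable plate stack, named as non-working, that hands out plates from the top to a grabbing player.
; On BeginPlay it spawns a column of physics-free BP_Plate actors attached at ObjectPlace, using DefaultAmount as both count and vertical spacing.
; GrabDrop checks whether the last plate in the array can be grabbed, then calls Grab, which forwards to that plate and removes it from the array.
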(event EventBeginPlay
  (CallFunction|InitializePlate))

(event EventGrabDrop
  (params (Player :type BP%20Character%20Object%20Reference))
  (bind _plates (Variables|Default|GetPlates))
  (if (Utilities|Array|IsNotEmpty (Variables|Default|GetPlates))
    (if (Default|CanbeGrabbed (Utilities|Array|Get(acopy) _plates (Utilities|Array|LastIndex _plates)) Player)
      (Default|Grab (Variables|Default|GetTarget) Player))))

(event EventGrab
  (params (player :type BP%20Character%20Object%20Reference))
  (bind _plates (Variables|Default|GetPlates))
  (bind _returnvalue (Utilities|Array|LastIndex _plates))
  (bind _output (Utilities|Array|Get(acopy) _plates _returnvalue))
  (Default|Grab _output player)
  (Utilities|Array|RemoveItem _plates _output))

(fn ConstructionScript
  (|CallParentFunction))

(fn InitializePlate
  (bind _objectplace (Variables|Default|GetObjectPlace))
  (bind _returnvalue (Transformation|GetWorldLocation _objectplace))
  (for _index (range 1 (Variables|PlateStack|GetdefaultAmount))
    (bind _returnvalue_2 (Game|SpawnActorfromClass "/Game/GameData/Blueprints/Interactable/KitchenWare/BP_Plate.BP_Plate_C" (Math|Transform|MakeTransform (Math|Vector|MakeVector (.x _returnvalue) (.y _returnvalue) (+ (.z _returnvalue) (* (Variables|PlateStack|GetdefaultAmount) (- _index 1))))) "Undefined" "MultiplyWithRoot" 0 0))
    (Default|RemovePhysics _returnvalue_2)
    (Transformation|AttachComponentToComponent _returnvalue_2 (Variables|Default|GetObjectPlace) "None" "KeepWorld" "KeepWorld" "KeepWorld" true)
    (Utilities|Array|Add (Variables|Default|GetPlates) _returnvalue_2)))