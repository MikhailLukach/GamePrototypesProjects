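; Pickup area actor where the player hands in a filled plate to complete the current order in a prison cooking game.
; It checks the plate's ingredients against recipes for the BP_OrderManager's order number, grading the meal as great, half-subpar, subpar or wrong.
; The grade and whether the customer is a guard drive sound effects and changes to cigars, unrest and sentence.
; The plate is then destroyed and the order marked inactive.
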(event Custom|PlayGreatMeal
  ;[1 1 1] Custom events to play needed soundeffects
  (bind _outactors (Actor|GetAllActorsOfClass "/Game/MySoundEffectPlayer.MySoundEffectPlayer_C"))
  (Class|SoundEffectPlayer|PlaySoundEffect (Utilities|Array|Get(acopy) _outactors) "/Game/GameData/WAVs/SW_SuperCorrectMeal.SW_SuperCorrectMeal" (Transformation|GetActorLocation)))

(event Custom|PlayDecentMeal
  ;[1 1 1] Custom events to play needed soundeffects
  (bind _outactors (Actor|GetAllActorsOfClass "/Game/MySoundEffectPlayer.MySoundEffectPlayer_C"))
  (Class|SoundEffectPlayer|PlaySoundEffect (Utilities|Array|Get(acopy) _outactors) "/Game/GameData/WAVs/SW_DecentMeal.SW_DecentMeal" (Transformation|GetActorLocation)))

(event Custom|PlayBadMeal
  ;[1 1 1] Custom events to play needed soundeffects
  (bind _outactors (Actor|GetAllActorsOfClass "/Game/MySoundEffectPlayer.MySoundEffectPlayer_C"))
  (Class|SoundEffectPlayer|PlaySoundEffect (Utilities|Array|Get(acopy) _outactors) "/Game/GameData/WAVs/SW_WrongMeal.SW_WrongMeal" (Transformation|GetActorLocation)))

(event EventBeginPlay
  ;[1 1 1] Sets the possible orders that can be called into a array
  (Variables|Default|SetPossibleOrders (Utilities|Array|MakeArray (Variables|TypesOfRecipes|GetMeatAndVeg) (Variables|TypesOfRecipes|GetMeat) (Variables|TypesOfRecipes|GetVeg))))

(event Collision|EventActorBeginOverlap
  (params (OtherActor :type Actor%20Object%20Reference)))

(event EventTick
  (params (DeltaSeconds :type Float%20%28single-precision%29)))

(event EventGrabDrop
  (params (Player :type BP%20Character%20Object%20Reference))
  ;[1 1 1] Sets initial values and checks whether given plate is empty, only occupied plates can be taken in
  (Variables|Default|SetIsHalfSubparRecipe false)
  (Variables|Default|SetIsSubparRecipe false)
  (bind _outactors (Actor|GetAllActorsOfClass "/Game/GameData/Blueprints/BP_OrderManager.BP_OrderManager_C"))
  (bind _asbp_plate (Utilities|Casting|CastToBP_Plate (.GrabbedObject (Default|GetGrabbedObject Player))))
  (if (not (Default|IsEmpty _asbp_plate))
    ;[1 1 1] Performs increments/decrements to systems based on what quality of meal has been given it
    (bind _correct (CallFunction|CheckifSubparRecipe _asbp_plate (Variables|/Game/GameData/Blueprints/BP_OrderManager.BP_OrderManager_C|GetorderNum (Utilities|Array|Get(acopy) _outactors))))
    (if _correct
      (if (Variables|Default|GetIsSubparRecipe)
        (CallFunction|PlayDecentMeal)
        (bind _outactors_2 (Actor|GetAllActorsOfClass "/Game/GameData/Blueprints/BP_OrderManager.BP_OrderManager_C"))
        (if (Variables|/Game/GameData/Blueprints/BP_OrderManager.BP_OrderManager_C|GetisGuard (Utilities|Array|Get(acopy) _outactors_2))
          (Default|IncrementSentence Player)
          (else
            (Default|IncrementPrisonUnrest Player)
            (Default|IncrementHalfCigars Player)))
        (elif (Variables|Default|GetIsHalfSubparRecipe)
          (CallFunction|PlayDecentMeal)
          (bind _outactors_3 (Actor|GetAllActorsOfClass "/Game/GameData/Blueprints/BP_OrderManager.BP_OrderManager_C"))
          (if (Variables|/Game/GameData/Blueprints/BP_OrderManager.BP_OrderManager_C|GetisGuard (Utilities|Array|Get(acopy) _outactors_3))
            (Default|IncrementSentence Player)
            (else
              (Default|IncrementHalfPrisonUnrest Player)))
          (Default|IncrementHalfCigars Player)
          (else
            (CallFunction|PlayGreatMeal)
            (Default|IncrementCigars Player)
            (Default|DecrementPrisonUnrest Player)
            (Development|PrintString "Hello" false false)
            (bind _outactors_4 (Actor|GetAllActorsOfClass "/Game/GameData/Blueprints/BP_OrderManager.BP_OrderManager_C"))
            (if (Variables|/Game/GameData/Blueprints/BP_OrderManager.BP_OrderManager_C|GetisGuard (Utilities|Array|Get(acopy) _outactors_4))
              (Default|DecrementSentence Player)))))
      ;[1 1 1] Destroys the plate and all objects on it, sets that order has been completed
      (Actor|DestroyActor _asbp_plate)
      (bind _outactors_5 (Actor|GetAllActorsOfClass "/Game/GameData/Blueprints/BP_OrderManager.BP_OrderManager_C"))
      (Variables|/Game/GameData/Blueprints/BP_OrderManager.BP_OrderManager_C|SetactiveOrder (Utilities|Array|Get(acopy) _outactors_5) false)
      (else
        ;[1 1 1] Increment and decrement of game systems for a completely wrong meal
        (CallFunction|PlayBadMeal)
        (Default|IncrementPrisonUnrest Player)
        (Development|PrintString "Hello" false false)
        (bind _outactors_6 (Actor|GetAllActorsOfClass "/Game/GameData/Blueprints/BP_OrderManager.BP_OrderManager_C"))
        (if (Variables|/Game/GameData/Blueprints/BP_OrderManager.BP_OrderManager_C|GetisGuard (Utilities|Array|Get(acopy) _outactors_6))
          (Default|IncrementSentence Player))
        (Actor|DestroyActor _asbp_plate)
        (Actor|GetAllActorsOfClass "/Game/GameData/Blueprints/BP_OrderManager.BP_OrderManager_C")
        (bind _outactors_7 (Actor|GetAllActorsOfClass "/Game/GameData/Blueprints/BP_OrderManager.BP_OrderManager_C"))
        (Variables|/Game/GameData/Blueprints/BP_OrderManager.BP_OrderManager_C|SetactiveOrder (Utilities|Array|Get(acopy) _outactors_7) false)))))

(fn ConstructionScript)

(fn CheckifSubparRecipe
  (params (PlateIngredients :type BP%20Plate%20Object%20Reference) (OrderNum :type Integer))
  (switch int OrderNum
    (:0
      (if (Default|Check (Variables|TypesOfRecipes|GetMeatAndVeg) (Default|GetIngredients PlateIngredients))
        (return true)
        (elif (or (Default|Check (Variables|TypesOfRecipes|GetSubparMeatAndVeg) (Default|GetIngredients PlateIngredients)) (Default|Check (Variables|TypesOfRecipes|GetMeatAndSubparVeg) (Default|GetIngredients PlateIngredients)))
          (Variables|Default|SetIsHalfSubparRecipe true)
          (return true)
          (elif (Default|Check (Variables|TypesOfRecipes|GetSubparMeatAndSubparVeg) (Default|GetIngredients PlateIngredients))
            (Variables|Default|SetIsSubparRecipe true)
            (return true)
            (else
              (return false))))))
    (:1
      (if (Default|Check (Variables|TypesOfRecipes|GetMeat) (Default|GetIngredients PlateIngredients))
        (return true)
        (elif (Default|Check (Variables|TypesOfRecipes|GetSubparMeat) (Default|GetIngredients PlateIngredients))
          (Variables|Default|SetIsSubparRecipe true)
          (return true)
          (else
            (return false)))))
    (:2
      (if (Default|Check (Variables|TypesOfRecipes|GetVeg) (Default|GetIngredients PlateIngredients))
        (return true)
        (elif (Default|Check (Variables|TypesOfRecipes|GetSubparVeg) (Default|GetIngredients PlateIngredients))
          (Variables|Default|SetIsSubparRecipe true)
          (return true)
          (else
            (return false)))))))

(fn TryGrab
  (params (Player :type BP%20Character%20Object%20Reference))
  (return false))