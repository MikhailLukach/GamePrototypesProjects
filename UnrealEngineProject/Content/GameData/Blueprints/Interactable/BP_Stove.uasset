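; BP_Stove is an interactable stove that cooks the pan placed on it.
; It extends its parent's Place and Grab events, sending CookMessage to the PlacedObject to start cooking after placement and to stop it before the parent grab runs.
; Grabbing also stops the controlled sound effect on the first MySoundEffectPlayer actor found in the level.
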(event EventGrab
  (params (player :type BP%20Character%20Object%20Reference))
  ;[1 1 1] Stop cook process when pick up pan of stove
  (Class|BPICookingPlate|Cook(Message) (Variables|Default|GetplacedObject) false)
  (|CallParentFunction player)
  (bind _outactors (Actor|GetAllActorsOfClass "/Game/MySoundEffectPlayer.MySoundEffectPlayer_C"))
  (Class|SoundEffectPlayer|StopSoundEffectControlled (Utilities|Array|Get(acopy) _outactors)))

(event EventPlace
  (params (player :type BP%20Character%20Object%20Reference) (objectToPlace :type BP%20Grabable%20Object%20Reference))
  ;[1 1 1] Start cook process when pan is placed on stove
  (|CallParentFunction player objectToPlace)
  (Class|BPICookingPlate|Cook(Message) (Variables|Default|GetplacedObject) true))

(fn ConstructionScript
  (|CallParentFunction))