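; Interactable table with a cutting board where a player slices a placed food item.
; Interact checks that the food can be sliced, changes its state, plays a cutting sound and marks the player as interacting.
; Tick advances Progress at SlicingSpeed, printing it on screen, then ends the interaction and sets the food's next state.
; Interrupted slicing keeps its progress, and grab/drop works only before slicing starts or after it finishes.
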(event EventBeginPlay
  (|CallParentFunction) ; This node is disabled and will not be called.\nDrag off pins to build functionality.
)

(event Collision|EventActorBeginOverlap
  (params (OtherActor :type Actor%20Object%20Reference))
  (|CallParentFunction OtherActor) ; This node is disabled and will not be called.\nDrag off pins to build functionality.
)

(event EventTick
  (params (DeltaSeconds :type Float%20%28single-precision%29))
  ;[1 1 1] Updates the slicing when the player is interacting with the cutting board
  (|CallParentFunction DeltaSeconds)
  (if (Variables|Default|GetisInteracting)
    (bind _output_get (Variables|Default|Setprogress (Math|Interpolation|FInterptoConstant (Variables|Default|Getprogress) 1.0 DeltaSeconds (Variables|Settings|GetslicingSpeed))))
    (Development|PrintString (Utilities|String|ToString(Float) _output_get) true true "(R=0.000000,G=0.660000,B=1.000000,A=1.000000)" DeltaSeconds)
    (if (== (Variables|Default|Getprogress) 1.0)
      (CallFunction|StopInteraction)
      (bind _asbp_food_item (Utilities|Casting|CastToBP_FoodItem (Variables|Default|GetplacedObject)))
      (Default|SetState _asbp_food_item "NewEnumerator2"))))

(event EventGrabDrop
  (params (Player :type BP%20Character%20Object%20Reference))
  ;[1 1 1] Grabs the object of the cutting board and resets the progress
  (if (CallFunction|CanGrabObject)
    (|CallParentFunction Player)
    (Variables|Default|Setprogress 0.0)))

(event EventInteract
  (params (Player :type BP%20Character%20Object%20Reference))
  ;[1 1 1] Setsthat the player is interacting with the cutting board and updates the state of the object to being sliced
  (bind _asbp_food_item (Utilities|Casting|CastToBP_FoodItem (Variables|Default|GetplacedObject)))
  (if (Default|CanbeSliced _asbp_food_item)
    (Default|SetState _asbp_food_item "NewEnumerator1")
    (bind _outactors (Actor|GetAllActorsOfClass "/Game/MySoundEffectPlayer.MySoundEffectPlayer_C"))
    (Class|SoundEffectPlayer|PlaySoundEffect (Utilities|Array|Get(acopy) _outactors) "/Game/GameData/WAVs/SW_CuttingSoundEffect.SW_CuttingSoundEffect" (Transformation|GetActorLocation))
    (Default|SetIsInteracting Player true self)
    (Variables|Default|SetinteractingPlayer Player)
    (Variables|Default|SetisInteracting true)))

(event EventStopInteraction
  ;[1 1 1] Sets that player has stopped interacting with cutting board
  (Variables|Default|SetisInteracting false)
  (Default|SetIsInteracting (Variables|Default|GetinteractingPlayer) false))

(fn ConstructionScript
  (|CallParentFunction))

(fn CanGrabObject
  (return (or (== (Variables|Default|Getprogress) 0.0) (== (Variables|Default|Getprogress) 1.0))))