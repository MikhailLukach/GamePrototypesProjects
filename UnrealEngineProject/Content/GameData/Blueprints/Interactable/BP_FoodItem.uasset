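; BP_FoodItem is a grabbable ingredient whose meshes come from a FoodItemAsset.
; SetState swaps the mesh across raw, slicing, sliced, on-plate and cooked states, and CanBeSliced allows cutting only cutable items that are raw or mid-slice.
; Grab puts the item in an empty-handed player's hands, or asks the held object to add it.
; CanBeGrabbed permits that only with empty hands or kitchenware that has space.
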(event Custom|SetState
  (params (State :type BPE_FoodItemState%20Enum :default "NewEnumerator0"))
  (bind _fooditemasset (Variables|Default|GetFoodItemAsset))
  ;[1 1 1] Sets the state to the food item that is needed
  (bind _output_get (Variables|Default|SetState State))
  (Components|StaticMesh|SetStaticMesh (Variables|Character|GetMesh) (Utilities|Select :Index _output_get :NewEnumerator0 (Variables|/Game/GameData/Blueprints/AssetTypes/DA_Food_Item_BP.DA_Food_Item_BP_C|GetUncutMesh _fooditemasset) :NewEnumerator1 (Variables|/Game/GameData/Blueprints/AssetTypes/DA_Food_Item_BP.DA_Food_Item_BP_C|GetBeingCutMesh _fooditemasset) :NewEnumerator2 (Variables|/Game/GameData/Blueprints/AssetTypes/DA_Food_Item_BP.DA_Food_Item_BP_C|GetBeenCutMesh _fooditemasset) :NewEnumerator3 (Variables|/Game/GameData/Blueprints/AssetTypes/DA_Food_Item_BP.DA_Food_Item_BP_C|GetOnPlateMesh _fooditemasset) :NewEnumerator4 (Variables|/Game/GameData/Blueprints/AssetTypes/DA_Food_Item_BP.DA_Food_Item_BP_C|GetCookedMesh _fooditemasset))))

(event EventBeginPlay
  ;[1 1 1] Calls BeginPlay from Grabable parent and sets initial mesh of food item
  (|CallParentFunction)
  (Components|StaticMesh|SetStaticMesh (Variables|Character|GetMesh) (Variables|/Game/GameData/Blueprints/AssetTypes/DA_Food_Item_BP.DA_Food_Item_BP_C|GetUncutMesh (Variables|Default|GetFoodItemAsset))))

(event Collision|EventActorBeginOverlap
  (params (OtherActor :type Actor%20Object%20Reference))
  (|CallParentFunction OtherActor) ; This node is disabled and will not be called.\nDrag off pins to build functionality.
)

(event EventTick
  (params (DeltaSeconds :type Float%20%28single-precision%29))
  (|CallParentFunction DeltaSeconds) ; This node is disabled and will not be called.\nDrag off pins to build functionality.
)

(event EventGrab
  (params (player :type BP%20Character%20Object%20Reference))
  (bind (_returnvalue _grabbedobject) (Default|GetGrabbedObject player))
  ;[1 1 1] Grabs food item either to the player's hands or the plate they are holding
  (Variables|Default|SetPerformMove false)
  (CallFunction|RemovePhysics)
  (if _returnvalue
    (Class|BPIDish|TryAddItem(Message) _grabbedobject self)
    (else
      (Default|Grab player self)
      (Development|PrintString (Utilities|GetDisplayName (Variables|Default|GetFoodItemAsset)) false false))))

(fn ConstructionScript
  (|CallParentFunction))

(fn CanbeSliced
  (return (and (Variables|Default|GetIsCutable) (Utilities|Select :Index (Variables|Default|GetState) :NewEnumerator0 true :NewEnumerator1 true :NewEnumerator2 false :NewEnumerator3 false :NewEnumerator4 false))))

(fn CanbeGrabbed
  (params (player :type BP%20Character%20Object%20Reference))
  (bind (_returnvalue _grabbedobject) (Default|GetGrabbedObject player))
  (if (not _returnvalue)
    (return true)
    (else
      (bind _asbp_kitchen_ware (Utilities|Casting|CastToBP_KitchenWare _grabbedobject)
        (:then
          (return (Default|HasPlace _asbp_kitchen_ware)))
        (:CastFailed
          (return false))))))