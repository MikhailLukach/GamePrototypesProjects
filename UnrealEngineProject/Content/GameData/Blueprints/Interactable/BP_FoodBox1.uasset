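; Interactable food box that sells veggie ingredients to the player for cigs.
; GrabDrop checks the player can afford a veggie, then plays a buying sound through the level's MySoundEffectPlayer.
; With nothing placed and empty hands, it spawns a BP_FoodItem from its FoodItemAsset, deducts the price and hands it over.
; A grabbable placed object or an already held item defers to the parent GrabDrop without charging.
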(event EventGrabDrop
  (params (Player :type BP%20Character%20Object%20Reference))
  ;[1 1 1] Spawns veggie ingredient in to player's hands when they interact with the food box and have enough cigs to purchase the veggie
  (bind _enough (Default|CheckifEnoughforVeg Player))
  (if _enough
    (bind _outactors (Actor|GetAllActorsOfClass "/Game/MySoundEffectPlayer.MySoundEffectPlayer_C"))
    (Class|SoundEffectPlayer|PlaySoundEffect (Utilities|Array|Get(acopy) _outactors) "/Game/GameData/WAVs/SW_BuyingSoundEffect.SW_BuyingSoundEffect" (Transformation|GetActorLocation))
    (bind _placedobject (Variables|Default|GetplacedObject)
      (:then
        (if (Default|CanbeGrabbed _placedobject Player)
          (|CallParentFunction Player :!label _label)))
      (:else
        (if (.ReturnValue (Default|GetGrabbedObject Player))
          (goto _label)
          (else
            (bind _returnvalue (Game|SpawnActorfromClass "/Game/GameData/Blueprints/Interactable/BP_FoodItem.BP_FoodItem_C" (Transformation|GetActorTransform) "Undefined" "MultiplyWithRoot" 0 true (Variables|FoodBox|GetfoodItemAsset) 0))
            (Default|DecrementVegPrice Player)
            (Default|GrabDrop _returnvalue Player)))))))

(fn ConstructionScript
  (|CallParentFunction))