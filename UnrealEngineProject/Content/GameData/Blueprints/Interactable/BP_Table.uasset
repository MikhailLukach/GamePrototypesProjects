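; BP_Table is an interactable table that holds one object at its ObjectPlace component, optionally spawning a default one on BeginPlay.
; GrabDrop places the player's held object when the table is empty, otherwise it attempts a grab.
; Placing strips physics, attaches the object and calls its MoveToPlace.
; Grabbing defers to the placed object's TryGrab and clears the slot only on success.
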(event Custom|Grab
  (params (player :type BP%20Character%20Object%20Reference))
  ;[1 1 1] performs grab itself
  (Variables|Table|SetplacedObject 0))

(event Custom|Place
  (params (player :type BP%20Character%20Object%20Reference) (objectToPlace :type BP%20Grabable%20Object%20Reference))
  ;[1 1 1] Places object on the table
  (CallFunction|AttachObject objectToPlace)
  (Variables|/Game/GameData/Blueprints/BP_Character.BP_Character_C|SetgrabbedObject player 0))

(event EventBeginPlay
  ;[1 1 1] Allows to set an object that needs to initially spawn on the table
  (bind _defaultplacedobjectclass (Variables|Table|GetdefaultPlacedObjectClass)
    (:then
      (bind _returnvalue (Game|SpawnActorfromClass _defaultplacedobjectclass (Transformation|GetWorldTransform (Variables|Default|GetObjectPlace)) "AlwaysSpawn" "MultiplyWithRoot" 0 0))
      (CallFunction|AttachObject _returnvalue))
    (:else)))

(event Collision|EventActorBeginOverlap
  (params (OtherActor :type Actor%20Object%20Reference)))

(event EventTick
  (params (DeltaSeconds :type Float%20%28single-precision%29)))

(event EventGrabDrop
  (params (Player :type BP%20Character%20Object%20Reference))
  (bind (_returnvalue _grabbedobject) (Default|GetGrabbedObject Player))
  ;[1 1 1] Grabs object of the table or places object on the table when the player interacts with it
  (if _returnvalue
    (Variables|Table|GetplacedObject
      (:then
        (CallFunction|TryGrab Player))
      (:else
        (CallFunction|Place Player _grabbedobject)))
    (else
      (CallFunction|TryGrab Player))))

(fn ConstructionScript)

(fn AttachObject
  (params (ObjectToPlace :type BP%20Grabable%20Object%20Reference))
  (bind _output_get (Variables|Table|SetplacedObject ObjectToPlace))
  (Default|RemovePhysics _output_get)
  (Transformation|AttachComponentToComponent (Variables|Table|GetplacedObject) (Variables|Default|GetObjectPlace) "None" "KeepWorld" "KeepWorld" "KeepWorld" true)
  (Default|MovetoPlace (Variables|Table|GetplacedObject)))

(fn TryGrab
  (params (Player :type BP%20Character%20Object%20Reference))
  (bind _placedobject (Variables|Table|GetplacedObject)
    (:then
      (bind _grabbed (Default|TryGrab _placedobject Player))
      (if _grabbed
        (CallFunction|Grab Player)
        (return true)
        (else
          (return false))))
    (:else
      (return false))))