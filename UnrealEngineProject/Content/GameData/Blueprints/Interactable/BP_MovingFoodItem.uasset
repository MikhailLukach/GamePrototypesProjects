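; Interactable food item that periodically hops to a random nearby spot.
; BeginPlay starts a looping timer calling RandomRoam, which acts only while PerformMove is set and State is not one particular value.
; It offsets a random navigable point near the actor in X/Y, then uses a swept SetActorLocation so blocking objects stop the move.
; A debug print rolls its own random offsets, so it need not match the actual destination.
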(event Custom|RandomRoam
  ;[1 1 1] Performs a random roam to a new location and avoid teleporting to a preoccupied location
  (if (Variables|Default|GetPerformMove)
    (if (not (Utilities|Enum|Equal(Enum) (Variables|Default|GetState) "NewEnumerator2"))
      (bind _randomlocation (Class|NavigationSystemV1|GetRandomLocationinNavigableRadius (Transformation|GetActorLocation self) 1e+01 0 0))
      (Development|PrintString (Utilities|String|ToString(Vector) (Math|Vector|MakeVector (+ (.x _randomlocation) (Math|Random|RandomFloatinRange -7e+01 7e+01)) (+ (.y _randomlocation) (Math|Random|RandomFloatinRange -7e+01 7e+01)) (.z _randomlocation))))
      (Transformation|SetActorLocation self (Math|Vector|MakeVector (+ (.x _randomlocation) (Math|Random|RandomFloatinRange -7e+01 7e+01)) (+ (.y _randomlocation) (Math|Random|RandomFloatinRange -7e+01 7e+01)) (.z _randomlocation)) true false))))

(event EventBeginPlay
  ;[1 1 1] Sets a timer so the movement actions can follow it
  (Utilities|Time|SetTimerbyFunctionName 0 "RandomRoam" 2.0 true)
  (|CallParentFunction))

(event Collision|EventActorBeginOverlap
  (params (OtherActor :type Actor%20Object%20Reference))
  (|CallParentFunction OtherActor) ; This node is disabled and will not be called.\nDrag off pins to build functionality.
)

(event EventTick
  (params (DeltaSeconds :type Float%20%28single-precision%29))
  (|CallParentFunction DeltaSeconds) ; This node is disabled and will not be called.\nDrag off pins to build functionality.
)

(fn ConstructionScript
  (|CallParentFunction))