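; Kitchen plate interactable that holds food items and reports their contents as recipe ingredients.
; TryAddItem extends the parent's add logic, returning success for raw, sliced or cooked food and switching sliced food to an on-plate state.
; GetIngredients tallies held items into a map keyed by food asset, storing an amount and the first recorded state for each.
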(event EventBeginPlay
  (|CallParentFunction) ; This node is disabled and will not be called.\nDrag off pins to build functionality.
)

(event Collision|EventActorBeginOverlap
  (params (OtherActor :type Actor%20Object%20Reference))
  (|CallParentFunction OtherActor) ; This node is disabled and will not be called.\nDrag off pins to build functionality.
)

(event EventTick
  (params (DeltaSeconds :type Float%20%28single-precision%29))
  (|CallParentFunction DeltaSeconds) ; This node is disabled and will not be called.\nDrag off pins to build functionality.
)

(fn ConstructionScript
  (|CallParentFunction))

(fn GetIngredients
  ;[1 1 1] Returns the current ingredients that are on any plate.
  (for _array_element (Variables|Default|Getitems)
    (bind _output_get (LocalVariables|SetfoodItem _array_element))
    (if (.ReturnValue (Utilities|Map|Find (LocalVariables|GetplateIngredients) (Variables|/Game/GameData/Blueprints/Interactable/BP_FoodItem.BP_FoodItem_C|GetFoodItemAsset _output_get)))
      (Utilities|Map|Add (LocalVariables|GetplateIngredients) (Variables|/Game/GameData/Blueprints/Interactable/BP_FoodItem.BP_FoodItem_C|GetFoodItemAsset (LocalVariables|GetfoodItem)) (Utilities|Struct|MakeBPS_RecipeIngredient (.state (.Value (Utilities|Map|Find (LocalVariables|GetplateIngredients) (Variables|/Game/GameData/Blueprints/Interactable/BP_FoodItem.BP_FoodItem_C|GetFoodItemAsset _output_get)))) (+ (.amount (.Value (Utilities|Map|Find (LocalVariables|GetplateIngredients) (Variables|/Game/GameData/Blueprints/Interactable/BP_FoodItem.BP_FoodItem_C|GetFoodItemAsset _output_get)))) 1)))
      (else
        (Utilities|Map|Add (LocalVariables|GetplateIngredients) (Variables|/Game/GameData/Blueprints/Interactable/BP_FoodItem.BP_FoodItem_C|GetFoodItemAsset (LocalVariables|GetfoodItem)) (Utilities|Struct|MakeBPS_RecipeIngredient (Variables|/Game/GameData/Blueprints/Interactable/BP_FoodItem.BP_FoodItem_C|GetState (LocalVariables|GetfoodItem)) 1)))))
  (return (LocalVariables|GetplateIngredients)))

(fn TryAddItem
  (params (foodItem :type BP%20Food%20Item%20Object%20Reference))
  ;[1 1 1] Adds object to the plate, only allows those that are raw, sliced or cooked.
  (bind _added (|CallParentFunction foodItem))
  (if _added
    (switch Utilities|FlowControl|Switch|SwitchonBPE_FoodItemState (Variables|/Game/GameData/Blueprints/Interactable/BP_FoodItem.BP_FoodItem_C|GetState foodItem)
      (:NewEnumerator0
        (Default|SetState foodItem "NewEnumerator0")
        (return true))
      (:NewEnumerator2
        (Default|SetState foodItem "NewEnumerator3")
        (return true))
      (:NewEnumerator4
        (Default|SetState foodItem "NewEnumerator4")
        (return true)))
    (else
      (return false))))