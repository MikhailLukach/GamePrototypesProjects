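; Cookware Blueprint that cooks the items placed on a pan, with frying and ready sounds from a sound effect player actor.
; Cook sets the cooking flag and, if items are present, starts a self-repeating delayed update that raises a score toward a per-item target.
; When cooking stops, the update plays the ready sound, sets only the first item's state to cooked and resets the score.
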(event Custom|UpdateCookingProcess
  (bind _items (Variables|Default|Getitems))
  (bind _output (Utilities|Array|Get(acopy) _items))
  ;[1 1 1] Keep updating the cook process by 1 if not done
  (bind _result (Math|Integer|IncrementInt (Variables|CookWare|GetcookingScore))
    (:%20%20
      (Development|PrintString (Utilities|String|ToString(Integer) _result))
      (Utilities|FlowControl|Delay 0.2)
      (if (>= (Variables|CookWare|GetcookingScore) (* (Variables|CookWare|GetcookingScorePerItem) (Utilities|Array|Length (Variables|Default|Getitems))))
        (Variables|CookWare|SetisCooking false))
      (if (Variables|CookWare|GetisCooking)
        (Development|PrintString (Utilities|String|ToString(Boolean) (Variables|CookWare|GetisCooking)) false)
        (CallFunction|UpdateCookingProcess)
        (else
          ;[1 1 1] Set state of object to cook once cooking process is complete + sound effect
          (Development|PrintString (Utilities|GetDisplayName _output) false)
          (bind _outactors (Actor|GetAllActorsOfClass "/Game/MySoundEffectPlayer.MySoundEffectPlayer_C"))
          (Class|SoundEffectPlayer|PlaySoundEffect (Utilities|Array|Get(acopy) _outactors) "/Game/GameData/WAVs/SW_Ready.SW_Ready" (Transformation|GetActorLocation))
          (Default|SetState _output "NewEnumerator4")
          (Variables|CookWare|SetcookingScore 0))))))

(event EventCook
  (params (enable :type Boolean))
  ;[1 1 1] Start cook process on object on pan + start cooking sound effect
  (Development|PrintString (Utilities|String|ToString(Integer) (Variables|CookWare|GetcookingScore)) false false)
  (bind _output_get (Variables|CookWare|SetisCooking enable))
  (if (and _output_get (Math|Conversions|ToBoolean(Integer) (Utilities|Array|Length (Variables|Default|Getitems))))
    (bind _outactors (Actor|GetAllActorsOfClass "/Game/MySoundEffectPlayer.MySoundEffectPlayer_C"))
    (Class|SoundEffectPlayer|PlaySoundEffectControlled (Utilities|Array|Get(acopy) _outactors) "/Game/GameData/WAVs/SW_PanFryindSound.SW_PanFryindSound")
    (CallFunction|UpdateCookingProcess)))

(fn ConstructionScript
  (|CallParentFunction))