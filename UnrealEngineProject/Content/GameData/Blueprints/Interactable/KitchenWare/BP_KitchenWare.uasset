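; BP_KitchenWare is an interactable plate-like container that holds food items up to a maximum count.
; TryAddItem accepts sliced, cooked or already-plated food, attaching it to FoodPlace.
; When parent grab handling fails, TryGrab adds the player's held food or transfers contents between two wares, filling this one if empty, otherwise the held one.
; Destroying the ware also destroys every item on it.
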(event Custom|OnDestroy
  (params (DestroyedActor :type Actor%20Object%20Reference))
  ;[1 1 1] Destroys every object on the plate
  (for _array_element (Variables|Dish|Getitems)
    (Actor|DestroyActor _array_element)))

(event EventBeginPlay
  ;[1 1 1] Sets destroy call of plate to also destroy every object on it
  (|CallParentFunction)
  (Game|BindEventtoOnDestroyed (EventDispatchers|CreateEvent :!event Custom|OnDestroy)))

(event Collision|EventActorBeginOverlap
  (params (OtherActor :type Actor%20Object%20Reference))
  (|CallParentFunction OtherActor) ; This node is disabled and will not be called.\nDrag off pins to build functionality.
)

(event EventTick
  (params (DeltaSeconds :type Float%20%28single-precision%29))
  (|CallParentFunction DeltaSeconds) ; This node is disabled and will not be called.\nDrag off pins to build functionality.
)

(fn ConstructionScript
  (|CallParentFunction))

(fn HasPlace
  ;[1 1 1] Checks whether there's space on the plate
  (return (< (Utilities|Array|Length (Variables|Dish|Getitems)) (Variables|Dish|GetmaxFoodCount))))

(fn IsEmpty
  (return (Utilities|Array|IsEmpty (Variables|Dish|Getitems))))

(fn TryGrab
  (params (Player :type BP%20Character%20Object%20Reference))
  (bind _grabbed (|CallParentFunction Player))
  (if _grabbed
    (return true)
    (else
      (bind _asbp_food_item (Utilities|Casting|CastToBP_FoodItem (Variables|/Game/GameData/Blueprints/BP_Character.BP_Character_C|GetgrabbedObject Player))
        (:then
          (bind _added (CallFunction|TryAddItem _asbp_food_item))
          (if _added
            (CallFunction|Grab Player)
            (return true)
            (else
              (return false))))
        (:CastFailed
          (bind _asbp_kitchen_ware (Utilities|Casting|CastToBP_KitchenWare (Variables|/Game/GameData/Blueprints/BP_Character.BP_Character_C|GetgrabbedObject Player))
            (:then
              (LocalVariables|SetPlayerKitchenWare _asbp_kitchen_ware)
              (if (CallFunction|IsEmpty)
                (bind _added_2 (CallFunction|TryAddItems (Variables|BP_KitchenWare_C|Getitems (LocalVariables|GetPlayerKitchenWare))))
                (if _added_2
                  (Utilities|Array|Clear (Variables|BP_KitchenWare_C|Getitems (LocalVariables|GetPlayerKitchenWare))))
                (return false)
                (else
                  (bind _added_3 (Default|TryAddItems (LocalVariables|GetPlayerKitchenWare) (Variables|Dish|Getitems)))
                  (if _added_3
                    (Utilities|Array|Clear (Variables|Dish|Getitems)))
                  (return false))))
            (:CastFailed
              (return false))))))))

(fn TryAddItem
  (params (foodItem :type BP%20Food%20Item%20Object%20Reference))
  ;[1 1 1] Sets object on the plate and sets its state to what is needed
  (if (CallFunction|HasPlace)
    (switch Utilities|FlowControl|Switch|SwitchonBPE_FoodItemState (Variables|/Game/GameData/Blueprints/Interactable/BP_FoodItem.BP_FoodItem_C|GetState foodItem)
      (:NewEnumerator2
        _)
      (:NewEnumerator3
        _)
      (:NewEnumerator4
        _))
    (Utilities|Array|Add (Variables|Dish|Getitems) foodItem)
    (Transformation|AttachComponentToComponent foodItem (Variables|Default|GetfoodPlace) "None" "KeepWorld" "KeepWorld" "KeepWorld" true)
    (Default|MovetoPlace foodItem)
    (return true)
    (else
      (return false))))

(fn TryAddItems
  (params (FoodItems :type Array%20of%20BP%20Food%20Item%20Object%20References))
  (if (<= (Utilities|Array|Length FoodItems) (- (Variables|Dish|GetmaxFoodCount) (Utilities|Array|Length (Variables|Dish|Getitems))))
    (for _array_element FoodItems
      (CallFunction|TryAddItem _array_element))
    (return true)
    (else
      (return false))))