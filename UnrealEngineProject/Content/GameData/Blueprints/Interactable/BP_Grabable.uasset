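; BP_Grabable is an interactable physics object that a player can pick up and drop.
; GrabDrop calls TryGrab, which grabs only if the player holds nothing, and prints the result.
; Grab disables physics and collision on the box and mesh, then passes itself to the player's Grab.
; Drop detaches it in world space and restores both; a MoveToPlace event calls MoveComponentTo on the root.
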(event Custom|Drop
  (bind _box (Variables|Default|GetBox))
  ;[1 1 1] Drops the object and enables its collisions
  (Variables|Default|SetPerformMove true)
  (Transformation|DetachFromActor "KeepWorld" "KeepWorld" "KeepWorld")
  (Physics|SetSimulatePhysics _box true)
  (Collision|SetCollisionEnabled _box "QueryAndPhysics")
  (Collision|SetCollisionEnabled (Variables|Default|GetMesh) "QueryAndPhysics"))

(event Custom|Grab
  (params (player :type BP%20Character%20Object%20Reference))
  ;[1 1 1] Performs the grab itself, removes physics to avoid any unnecessary collisions
  (Variables|Default|SetPerformMove false)
  (CallFunction|RemovePhysics)
  (Default|Grab player self))

(event Custom|MoveToPlace
  ;[1 1 1] Moves object to the necessary location
  (Components|MoveComponentTo (Variables|Transformation|GetRootComponent) "0, 0, 0" "0, 0, 0" false false 0.2 false))

(event EventBeginPlay)

(event Collision|EventActorBeginOverlap
  (params (OtherActor :type Actor%20Object%20Reference)))

(event EventTick
  (params (DeltaSeconds :type Float%20%28single-precision%29)))

(event EventGrabDrop
  (params (Player :type BP%20Character%20Object%20Reference))
  ;[1 1 1] Perform grab on the object and check whether it can be
  (bind _grabbed (CallFunction|TryGrab self Player))
  (Development|PrintString (Utilities|String|ToString(Boolean) _grabbed)))

(fn ConstructionScript)

(fn CanbeGrabbed
  (params (player :type BP%20Character%20Object%20Reference))
  (return (not (.ReturnValue (Default|GetGrabbedObject player)))))

(fn RemovePhysics
  (bind _box (Variables|Default|GetBox))
  (Physics|SetSimulatePhysics _box false)
  (Collision|SetCollisionEnabled _box "NoCollision")
  (Collision|SetCollisionEnabled (Variables|Default|GetMesh) "NoCollision"))

(fn TryGrab
  (params (Player :type BP%20Character%20Object%20Reference))
  ;[1 1 1] Checks whether object can be grabbed
  (if (CallFunction|CanbeGrabbed Player)
    (CallFunction|Grab Player)
    (return true)
    (else
      (return false))))