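; Order manager actor that generates timed meal orders from guards or prisoners and checks the game's win and lose conditions.
; Tick polls BP_Character, pausing with a lose screen at full PrisonUnrest or a win screen at zero SentenceAmount.
; It counts down order patience; expiry plays a wrong-meal sound, increments unrest and sentence, and replaces the order.
; The first order is always prisoner meat; later ones randomise type and origin, favouring prisoners, whenever ActiveOrder is false or patience expires.
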(event Custom|SetOrderOrigin
  ;[1 1 1] Decides whether order comes from guard or prisoner
  (if (>= (Math|Random|RandomFloatinRange 0.0 1e+02) 75.0)
    (Variables|Order|SetisGuard true)
    (else
      (Variables|Order|SetisGuard false))))

(event Custom|SetupOrder
  ;[1 1 1] Sets up new order
  (CallFunction|SetOrderOrigin)
  (CallFunction|SetOrderType)
  (CallFunction|ResetTimer))

(event Custom|CountdownTimerBar
  ;[1 1 1] Counts down the patience bar
  (Variables|Default|SetpatienceAmount (Math|Float|Clamp(Float) (- (Variables|Default|GetpatienceAmount) (Utilities|Time|GetWorldDeltaSeconds)) 0.0 (Variables|Default|GetpatienceAmount))))

(event Custom|SetOrderType
  ;[1 1 1] Decide what order type it is
  (switch int (Math|Random|RandomIntegerinRange 0 2)
    (:0
      (Variables|Default|SetorderNum 0))
    (:1
      (Variables|Default|SetorderNum 1))
    (:2
      (Variables|Default|SetorderNum 2))))

(event Custom|ResetTimer
  ;[1 1 1] Resets timer
  (Variables|Default|SetpatienceAmount 1e+02))

(event Custom|SetupStarterOrder
  ;[1 1 1] Sets up initial order so its always meat
  (Variables|Default|SetorderNum 1)
  (Variables|Order|SetisGuard false))

(event EventBeginPlay
  ;[1 1 1] Set initial order + timer
  (CallFunction|ResetTimer)
  (CallFunction|SetupStarterOrder)
  (Variables|Components|SetactiveOrder true))

(event EventTick
  (params (DeltaSeconds :type Float%20%28single-precision%29))
  ;[1 1 1] Control win and lose conditions
  (bind _outactors (Actor|GetAllActorsOfClass "/Game/GameData/Blueprints/BP_Character.BP_Character_C"))
  (if (== (Variables|/Game/GameData/Blueprints/BP_Character.BP_Character_C|GetprisonUnrest (Utilities|Array|Get(acopy) _outactors)) 1.0)
    (bind _returnvalue (UserInterface|CreateWidget "/Game/GameData/Blueprints/BPW_LoseScreen.BPW_LoseScreen_C"))
    (UserInterface|Viewport|AddtoViewport _returnvalue 0)
    (Game|SetGamePaused true)
    (elif (== (Variables|/Game/GameData/Blueprints/BP_Character.BP_Character_C|GetsentenceAmount (Utilities|Array|Get(acopy) _outactors)) 0)
      (bind _returnvalue_2 (UserInterface|CreateWidget "/Game/GameData/Blueprints/BPW_WonScreen.BPW_WonScreen_C"))
      (UserInterface|Viewport|AddtoViewport _returnvalue_2 0)
      (Game|SetGamePaused true)
      (else
        ;[1 1 1] Set new order after order hand in (correct + wrong)
        (if (Variables|Components|GetactiveOrder)
          (CallFunction|CountdownTimerBar)
          (if (<= (Variables|Default|GetpatienceAmount) 0.0)
            (bind _outactors_2 (Actor|GetAllActorsOfClass "/Game/MySoundEffectPlayer.MySoundEffectPlayer_C"))
            (Class|SoundEffectPlayer|PlaySoundEffect (Utilities|Array|Get(acopy) _outactors_2) "/Game/GameData/WAVs/SW_WrongMeal.SW_WrongMeal" (Transformation|GetActorLocation))
            (bind _outactors_3 (Actor|GetAllActorsOfClass "/Game/GameData/Blueprints/BP_Character.BP_Character_C"))
            (Default|IncrementPrisonUnrest (Utilities|Array|Get(acopy) _outactors_3))
            (Default|IncrementSentence (Utilities|Array|Get(acopy) _outactors_3))
            (CallFunction|SetupOrder)
            (Variables|Components|SetactiveOrder true))
          (else
            (CallFunction|SetupOrder)
            (Variables|Components|SetactiveOrder true)))))))

(fn ConstructionScript)